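; Goku actor that shows an energy beam attack, switching between charge and fire visuals based on CurrentState.
; Construction and Tick both refresh mesh visibility, particle activation and the charge light from that state.
; ChargeAmount scales the charge particles and drives light intensity through a power curve relative to its original brightness.
; Tick polls the ShouldFire flag, which switches to the firing state and triggers the fire particles once.
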(event EventBeginPlay)

(event EventActorBeginOverlap
  (params (OtherActor :type Actor%20Object%20Reference)))

(event EventTick
  (params (DeltaSeconds :type Float%20%28single-precision%29))
  (CallFunction|UpdateComponents)
  (if (Variables|BehaviorChanges|GetShould%20Fire)
    (CallFunction|FireBeam)))

(fn ConstructionScript
  (Variables|Behavior|SetFull%20Charge%20Light%20Intensity (Variables|/Script/Engine.LightComponentBase|GetIntensity (Variables|Default|GetCharge%20Light)))
  (CallFunction|UpdateComponents))

(fn UpdateComponents
  (bind _charge_amount (Variables|Behavior|GetCharge%20Amount))
  (bind _current_state (Variables|Behavior|GetCurrent%20State))
  (bind _current_state_2 (Variables|Behavior|GetCurrent%20State))
  (bind _returnvalue (Utilities|Enum|Equal(Enum) _current_state "NewEnumerator2"))
  (bind _returnvalue_2 (Utilities|Enum|Equal(Enum) _current_state_2 "NewEnumerator2"))
  (bind _returnvalue_3 (not _returnvalue_2))
  (Rendering|SetVisibility (Variables|Default|GetFire%20Mesh) (Utilities|Enum|Equal(Enum) (Variables|Behavior|GetCurrent%20State) "NewEnumerator2") false)
  (Rendering|SetVisibility (Variables|Default|GetCharge%20Mesh) (or (Utilities|Enum|Equal(Enum) (Variables|Behavior|GetCurrent%20State) "NewEnumerator0") (Utilities|Enum|Equal(Enum) (Variables|Behavior|GetCurrent%20State) "NewEnumerator1")) false)
  (Effects|Components|ParticleSystem|SetVectorParameter (Variables|Default|GetBeam%20Charge%20Particles) "Scale" (Math|Vector|MakeVector _charge_amount _charge_amount _charge_amount))
  (Components|Activation|SetActive _returnvalue_3 false)
  (Rendering|SetVisibility (Variables|Default|GetCharge%20Light) _returnvalue_3 false)
  (if (Math|Boolean|NotEqual(Boolean) (Components|Activation|IsActive (Variables|Default|GetBeam%20Particles)) _returnvalue)
    (Components|Activation|SetActive (Variables|Default|GetBeam%20Particles) _returnvalue false))
  (if (not (Utilities|Enum|Equal(Enum) (Variables|Behavior|GetCurrent%20State) "NewEnumerator2"))
    (Rendering|Components|Light|SetIntensity (Variables|Default|GetCharge%20Light) (* (Variables|Behavior|GetFull%20Charge%20Light%20Intensity) (Math|Float|Power (Variables|Behavior|GetCharge%20Amount) (Variables|Behavior|GetCharge%20Brightness%20Power))))))

(fn FireBeam
  (bind _fire_particles (Variables|Default|GetFire%20Particles))
  (Variables|Behavior|SetCurrent%20State "NewEnumerator2")
  (Variables|BehaviorChanges|SetShould%20Fire false)
  (Rendering|SetVisibility _fire_particles true false)
  (Components|Activation|Activate _fire_particles false)
  (Rendering|SetVisibility (Variables|Default|GetBeam%20Charge%20Particles) false false))