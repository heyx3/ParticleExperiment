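; WindController is an actor that publishes wind settings to materials and positions a dust particle emitter and a water surface.
; A shared update function runs from the Construction Script and every Tick, moving both components to their configured relative positions.
; It writes wind strength to the WindData Material Parameter Collection, along with the actor's world location as the wind source vector.
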(event EventTick
  (params (DeltaSeconds :type Float%20%28single-precision%29))
  (CallFunction|UpdateWindStuff false))

(fn ConstructionScript
  (CallFunction|UpdateWindStuff true))

(fn UpdateWindStuff
  (params (Is%20Construction%20Script? :type Boolean))
  (bind _returnvalue (Transformation|GetActorLocation))
  (bind (_x _y _z) (Math|Vector|BreakVector _returnvalue))
  (Transformation|SetRelativeLocation (Variables|Default|GetDust%20Particles) (Variables|Wind|GetDust%20Emitter%20Pos) false)
  (Transformation|SetRelativeLocation (Variables|Default|GetWater%20Surface) (Variables|Wind|GetWater%20Surface%20Pos) false)
  (Rendering|Material|SetScalarParameterValue "/Game/Materials/WindData.WindData" "Wind Strength" (Variables|Wind|GetWind%20Strength) :!class /Script/Engine.KismetMaterialLibrary)
  (Rendering|Material|SetVectorParameterValue "/Game/Materials/WindData.WindData" "Wind Source" (Utilities|Struct|MakeLinearColor _x _y _z 0.0) :!class /Script/Engine.KismetMaterialLibrary))